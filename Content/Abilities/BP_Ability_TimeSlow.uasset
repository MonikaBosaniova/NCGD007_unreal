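; BP_Ability_TimeSlow is a pickup that grants the player the time ability.
; On pickup, it casts the player character to BP_ThirdPersonCharacter and tints the PlayerSphere mesh's emissive material parameter blue.
; It then turns on the time ability flag, clears the levitation flag so the time ability replaces it, and destroys itself.
; The slowing effect itself is not implemented here.
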(event EventBeginPlay
  (|CallParentFunction) ; This node is disabled and will not be called.\nDrag off pins to build functionality.
)

(event Collision|EventActorBeginOverlap
  (params (OtherActor :type Actor%20Object%20Reference))
  (|CallParentFunction OtherActor) ; This node is disabled and will not be called.\nDrag off pins to build functionality.
)

(event EventTick
  (params (DeltaSeconds :type Float%20%28single-precision%29))
  (|CallParentFunction DeltaSeconds) ; This node is disabled and will not be called.\nDrag off pins to build functionality.
)

(event EventOnPickedUp
  (bind _asbp_third_person_character (Utilities|Casting|CastToBP_ThirdPersonCharacter (Game|GetPlayerCharacter 0)))
  (bind _asmesh_component (Utilities|Casting|CastToMeshComponent (Variables|/Game/ThirdPerson/Blueprints/BP_ThirdPersonCharacter.BP_ThirdPersonCharacter_C|GetPlayerSphere _asbp_third_person_character))
    (:then
      (Rendering|Material|SetVectorParameterValueonMaterials _asmesh_component "Emissive color 02" "0.000000,0.031452,2.625000")
      (Variables|/Game/ThirdPerson/Blueprints/BP_ThirdPersonCharacter.BP_ThirdPersonCharacter_C|SetHasTimeAbility _asbp_third_person_character true)
      (Variables|/Game/ThirdPerson/Blueprints/BP_ThirdPersonCharacter.BP_ThirdPersonCharacter_C|SetHasLevitationAbility _asbp_third_person_character false)
      (Actor|DestroyActor))
    (:CastFailed
      (Development|PrintString "Hello"))))

(fn ConstructionScript
  (|CallParentFunction))